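; PBP_TopView is a top-view camera pawn that the player moves and zooms.
; On BeginPlay it casts its controller to PCBP_TopView and adds the IMC_TopView Enhanced Input mapping context.
; Move input feeds AddMovementInput along the camera's right vector and its forward vector flattened to the ground plane.
; Zoom input adds a scaled offset to the SpringArm length, with no clamping.
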(event `self.ReceiveBeginPlay`
  (`self.SetMappingContext`))

(event `EnhancedInput|/Game/Blueprints/KeyMapping/IA_MoveCamera`
  (params (ActionValue :type "Vector2D Structure") (ElapsedSeconds :type "Float (double-precision)") (TriggeredSeconds :type "Float (double-precision)") (InputAction :type "InputAction Object Reference" :default "/Game/Blueprints/KeyMapping/IA_MoveCamera.IA_MoveCamera"))
  (bind (_x _y) (`KismetMathLibrary.BreakVector2D` ActionValue))
  (bind (_returnvalue_x _returnvalue_y) (`KismetMathLibrary.BreakVector` (`SceneComponent.GetForwardVector` (`self.Camera`))))
  ;[1 1 1] Camera 이동 제어
  (:`Triggered`
    (`self.AddMovementInput` (`SceneComponent.GetRightVector` (`self.Camera`)) _x)
    (`self.AddMovementInput` (`KismetMathLibrary.Normal` (`KismetMathLibrary.MakeVector` _returnvalue_x _returnvalue_y)) _y)))

(event `EnhancedInput|/Game/Blueprints/KeyMapping/IA_ZoomCamera`
  (params (ActionValue :type "Float (double-precision)") (ElapsedSeconds :type "Float (double-precision)") (TriggeredSeconds :type "Float (double-precision)") (InputAction :type "InputAction Object Reference" :default "/Game/Blueprints/KeyMapping/IA_ZoomCamera.IA_ZoomCamera"))
  (bind _springarm (`self.SpringArm`))
  ;[1 1 1] Camera Zoom 제어
  (:`Triggered`
    (set `SpringArmComponent.TargetArmLength` (+ (* ActionValue 10.0) (`SpringArmComponent.TargetArmLength` _springarm)) _springarm)))

(fn `SetMappingContext`
  (bind _aspcbp_top_view (cast `/Game/Blueprints/CameraMan/PCBP_TopView` (`self.GetController`)))
  (`EnhancedInputSubsystemInterface.AddMappingContext` (pcsubsystem `EnhancedInputLocalPlayerSubsystem` _aspcbp_top_view) "/Game/Blueprints/KeyMapping/IMC_TopView.IMC_TopView" 0 (struct)))

(fn `UserConstructionScript`)